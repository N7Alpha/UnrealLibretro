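; Arcade cabinet actor that runs a Libretro core with two tethered, grabbable light guns and a coin slot.
; On BeginPlay each gun gets a port and cable, and snaps back to its parent component's transform when dropped.
; A Dogecoin actor entering the slot briefly presses Start and Select on port 0 to join and insert credit.
; When the core is ready, each gun's label shows its controller description.
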(event `self.ReceiveBeginPlay`
  ;[1 1 1] Return gun to its spawned position when it is let go by a Player
  (`parent.ReceiveBeginPlay`)
  (for _index (range 2)
    (bind _aslibretro_arcade_gun_actor (cast `/UnrealLibretro/Blueprints/LibretroArcadeGunActor` (`|GetArrayItem` (`|MakeArray` (`ChildActorComponent.ChildActor` (`self.LeftGun`)) (`ChildActorComponent.ChildActor` (`self.RightGun`))) _index)))
    (add `LibretroGrabComponent.OnDropped` (`/UnrealLibretro/Blueprints/LibretroArcadeGunActor.GrabComponentSnap` _aslibretro_arcade_gun_actor) (delegate `Gun Dropped`))
    ;[1 1 1] (Cosmetic) Attach cables from Arcade cabinet to gun
    (`CableComponent.SetAttachEndToComponent` (`|GetArrayItem` (`|MakeArray` (`self.LeftGunWire`) (`self.RightGunWire`)) _index) (`/UnrealLibretro/Blueprints/LibretroArcadeGunActor.CableAttachLocation` _aslibretro_arcade_gun_actor) "None")
    (bind _output_get (set `/UnrealLibretro/Blueprints/LibretroArcadeGunActor.Port` _index _aslibretro_arcade_gun_actor))
    (`TextRenderComponent.K2_SetText` (`|GetArrayItem` (`|MakeArray` (`self.LeftGunControllerTextRender`) (`self.RightGunControllerTextRender`)) _output_get) (`KismetTextLibrary.Conv_StringToText` "Test"))))

(event `Gun Dropped`
  (params (GrabComponent :type "LibretroGrabComponent Object Reference"))
  (bind _returnvalue (`ActorComponent.GetOwner` GrabComponent))
  ;[1 1 1] Return gun to its spawned position when it is let go by a Player
  (`self.K2_SetActorTransform` _returnvalue (`SceneComponent.K2_GetComponentToWorld` (`self.GetParentComponent` _returnvalue)) false false))

(event `self.Coin Slot Collision.OnComponentBeginOverlap`
  (params (OverlappedComponent :type "PrimitiveComponent Object Reference") (OtherActor :type "Actor Object Reference") (OtherComp :type "PrimitiveComponent Object Reference") (OtherBodyIndex :type Integer) (bFromSweep :type Boolean) (SweepResult :type "HitResult Structure (by ref)"))
  (bind _libretrocoreinstance (`self.LibretroCoreInstance`))
  ;[1 1 1] Handle someone putting their coin into our slot
  (bind _asstatic_mesh_component (cast `StaticMeshComponent` OtherComp))
  (cast `/UnrealLibretro/Blueprints/LibretroDogeCoinActor` (`ActorComponent.GetOwner` _asstatic_mesh_component))
  (`LibretroCoreInstance.SetInputDigital` _libretrocoreinstance 0 true "JoypadStart") ; This is the player join button...
  (`LibretroCoreInstance.SetInputDigital` _libretrocoreinstance 0 true "JoypadSelect") ; and this is the insert coin button for mame
  (`KismetSystemLibrary.K2_SetTimerDelegate` (delegate `Release Start Button`) 0.1))

(event `Release Start Button`
  (bind _libretrocoreinstance (`self.LibretroCoreInstance`))
  ;[1 1 1] Handle someone putting their coin into our slot
  (`LibretroCoreInstance.SetInputDigital` _libretrocoreinstance 0 false "JoypadStart")
  (`LibretroCoreInstance.SetInputDigital` _libretrocoreinstance 0 false "JoypadSelect"))

(event `self.LibretroCoreInstance.OnCoreIsReady`
  (params (LibretroFramebuffer :type "TextureRenderTarget2D Object Reference") (AudioBuffer :type "SoundWave Object Reference"))
  (for _index (range 2)
    (bind (_id _description) (`LibretroCoreInstance.GetController` (`self.LibretroCoreInstance`) _index))
    (`TextRenderComponent.K2_SetText` (`|GetArrayItem` (`|MakeArray` (`self.LeftGunControllerTextRender`) (`self.RightGunControllerTextRender`)) _index) (`KismetTextLibrary.Conv_StringToText` _description))))

(fn `UserConstructionScript`
  (`parent.UserConstructionScript`))