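; Pawn for focused play of a Libretro-emulated game, routing the possessing player's input into a LibretroCoreInstance.
; On possession it connects the controller to the core with combined keyboard and gamepad bindings, forwarding keyboard input where possible.
; E disconnects port 0 and hands possession to PawnToPossessWhenUnpossessed.
; Mouse input rotates the spring-arm camera cosmetically, and the Colon key demonstrates setting a joypad button directly on the core.
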(event `Key|E`
  (params (Key :type "Key Structure"))
  ;[1 1 1] Unreal Delegates
  (:`Pressed`
    (`LibretroCoreInstance.DisconnectController` (`self.LibretroCoreInstance`) 0)
    (`Controller.Possess` (`Pawn.GetController`) (`self.PawnToPossessWhenUnpossessed`))))

(event `InputAxisKey|MouseY`
  (params (AxisValue :type "Float (single-precision)"))
  ;[1 1 1] Unreal Delegates
  ;;[1 1 1] (Cosmetic) Allows camera to rotate around pawn
  (`SceneComponent.K2_AddRelativeRotation` (`self.SpringArm`) (`KismetMathLibrary.MakeRotator` 0.0 AxisValue (`self.GetInputAxisKeyValue`)) false false))

(event `self.ReceivePossessed`
  (params (NewController :type "Controller Object Reference"))
  ;[1 1 1] Unreal Delegates
  (bind _asplayer_controller (cast `PlayerController` NewController))
  (`LibretroCoreInstance.ConnectController` (`self.LibretroCoreInstance`) _asplayer_controller 0 (`LibretroBlueprintFunctionLibrary.CombineInputMaps` (`|MakeMap` "X" "JoypadA" "Z" "JoypadB" "Up" "JoypadUp" "Down" "JoypadDown" "Left" "JoypadLeft" "Right" "JoypadRight" "RightShift" "JoypadSelect" "C" "JoypadX" "V" "JoypadY" "F" "JoypadL" "G" "JoypadR" "Enter" "JoypadStart" :!type "Key Structure" :!valuetype "ERetroDeviceID Enum") (`|MakeMap` "Gamepad_LeftX" "AnalogLeftX" "Gamepad_LeftY" "AnalogRightX" "Gamepad_RightX" "AnalogRightX" "Gamepad_RightY" "AnalogRightY" "Gamepad_FaceButton_Right" "JoypadA" "Gamepad_FaceButton_Left" "JoypadY" "Gamepad_FaceButton_Top" "JoypadX" "Gamepad_FaceButton_Left" "JoypadY" "Gamepad_Special_Right" "JoypadStart" "Gamepad_Special_Left" "JoypadSelect" "Gamepad_LeftTrigger" "JoypadL2" "Gamepad_RightTrigger" "JoypadR2" "Gamepad_LeftShoulder" "JoypadL" "Gamepad_RightShoulder" "JoypadR" "Gamepad_LeftThumbstick" "JoypadL3" "Gamepad_RightThumbstick" "JoypadR3" "Gamepad_DPad_Up" "JoypadUp" "Gamepad_DPad_Right" "JoypadRight" "Gamepad_DPad_Down" "JoypadDown" "Gamepad_DPad_Left" "JoypadLeft" :!type "Key Structure" :!valuetype "ERetroDeviceID Enum")) (delegate `Controller Disconnected`) true))

(event `Controller Disconnected`
  (params (PlayerController :type "PlayerController Object Reference") (Port :type Integer))
  ;[1 1 1] Unreal Delegates
)

(event `Key|Colon` :!enabledstate Disabled
  (params (Key :type "Key Structure"))
  (bind _libretrocoreinstance (`self.LibretroCoreInstance`))
  ;[1 1 1] Key Bindings for emulated game
  ;;[0.04519 0.4508 0.1651] You can set inputs corresponding to events directly this way now. This should be a lot more of a flexible way to do it although its more verbose. Be careful though if you set inputs this way axis bindings will be overridden if you use Connect Controller since axis values are polled every tick
  (:`Pressed`
    (`LibretroCoreInstance.SetInputDigital` _libretrocoreinstance 0 true "JoypadB"))
  (:`Released`
    (`LibretroCoreInstance.SetInputDigital` _libretrocoreinstance 0 false "JoypadB")))

(fn `UserConstructionScript`)