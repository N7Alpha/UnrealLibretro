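; LibretroHUD is a HUD Blueprint that draws an interact prompt in white text, positioned at the screen center.
; ShowInteractPromptForOneFrame sets a flag, which DrawHUD checks and clears after drawing InteractPromptText.
; The prompt therefore stays visible only while the event keeps being called each frame, with no separate hide call.
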(event `ShowInteractPromptForOneFrame`
  (set `self.ShouldShowInteractPrompt` true))

(event `self.ReceiveDrawHUD`
  (params (SizeX :type Integer) (SizeY :type Integer))
  (if (`self.ShouldShowInteractPrompt`)
    (`self.DrawText` (`self.InteractPromptText`) (struct :`R` 1.0 :`G` 1.0 :`B` 1.0 :`A` 1.0) (* (`KismetMathLibrary.Conv_IntToDouble` SizeX) 0.5) (* (`KismetMathLibrary.Conv_IntToDouble` SizeY) 0.5) null)
    (set `self.ShouldShowInteractPrompt` false)))

(fn `UserConstructionScript`
  (`parent.UserConstructionScript`))