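; Base actor for an in-world emulator screen that runs a libretro core, displaying its framebuffer on a mesh and routing its sound to an audio component.
; BeginPlay applies a dynamic screen material and optionally launches the core.
; Successful launch and framebuffer resizes update material UV scale, shift and rotation to match the frame's size, origin and orientation.
; Persistent actors save state on EndPlay and reload it after auto-launching.
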(event `self.LibretroCoreInstance.OnLaunchComplete`
  (params (LibretroFramebuffer :type "TextureRenderTarget2D Object Reference") (AudioBuffer :type "SoundWave Object Reference") (bSuccess :type Boolean))
  (bind _screenmaterialinstance (`self.ScreenMaterialInstance`))
  (bind _libretrocoreinstance (`self.LibretroCoreInstance`))
  (bind _rendertarget (`LibretroCoreInstance.RenderTarget` _libretrocoreinstance))
  (bind _bframebottomleftorigin (`LibretroCoreInstance.bFrameBottomLeftOrigin` _libretrocoreinstance))
  (bind _returnvalue (/ (`KismetMathLibrary.Conv_IntToDouble` (`LibretroCoreInstance.FrameHeight` _libretrocoreinstance)) (`KismetMathLibrary.Conv_IntToDouble` (`TextureRenderTarget2D.SizeY` _rendertarget))))
  (if bSuccess
    (`MaterialInstanceDynamic.SetTextureParameterValue` _screenmaterialinstance "EmulatorTexture" LibretroFramebuffer)
    ;[0.03434 0.03434 0.03434] Set parameters in material instance to possibly scale, shift, reflect, and rotate UV coordinates such that the frame drawn by the libretro core in our rendertarget i.e. If our mesh UV's cover from [0, 0] to [1, 1] then the mesh will be filled from edge to edge with the content of the framebuffer in a fixed likely right-side-up orientation. However you have to make sure the aspect ratio of the mesh matches the game's if you don't want the image to be stretched
    (`MaterialInstanceDynamic.SetScalarParameterValue` _screenmaterialinstance "UScale" (/ (`KismetMathLibrary.Conv_IntToDouble` (`LibretroCoreInstance.FrameWidth` _libretrocoreinstance)) (`KismetMathLibrary.Conv_IntToDouble` (`TextureRenderTarget2D.SizeX` _rendertarget))) :!label _label)
    (`MaterialInstanceDynamic.SetScalarParameterValue` _screenmaterialinstance "VScale" (select `bool` _bframebottomleftorigin :`false` _returnvalue :`true` (- 0.0 _returnvalue)))
    (`MaterialInstanceDynamic.SetScalarParameterValue` _screenmaterialinstance "RotationInCycles" (`LibretroCoreInstance.FrameRotation` _libretrocoreinstance))
    (if _bframebottomleftorigin
      (`MaterialInstanceDynamic.SetScalarParameterValue` _screenmaterialinstance "VShift" _returnvalue))))

(event `self.LibretroCoreInstance.OnCoreFrameBufferResize`
  ;[0.03434 0.03434 0.03434] Set parameters in material instance to possibly scale, shift, reflect, and rotate UV coordinates such that the frame drawn by the libretro core in our rendertarget i.e. If our mesh UV's cover from [0, 0] to [1, 1] then the mesh will be filled from edge to edge with the content of the framebuffer in a fixed likely right-side-up orientation. However you have to make sure the aspect ratio of the mesh matches the game's if you don't want the image to be stretched
  (goto _label))

(event `self.ReceiveBeginPlay`
  ;[0.03434 0.03434 0.03434] Unreal Delegates
  ;;[0.03434 0.03434 0.03434] Create our custom material that let's us shift uv's around since the actual drawn frame can end up in wacky positions and orientations in the framebuffer the above code to get around this is a testament to that
  (bind _returnvalue (`KismetMaterialLibrary.CreateDynamicMaterialInstance` (`self.ScreenMaterialParent`)))
  (bind _output_get (set `self.ScreenMaterialInstance` _returnvalue))
  (`PrimitiveComponent.SetMaterial` (`self.ScreenMesh`) 0 _output_get)
  (set `LibretroCoreInstance.AudioComponent` (`self.Audio`) (`self.LibretroCoreInstance`)) ; This tells the core instance where it should play sound from
  (if (`self.InitiallyTurnedOn`)
    (`LibretroCoreInstance.Launch` (`self.LibretroCoreInstance`)) ; This starts the process of loading the core which will eventually trigger "On Launch Complete" in the child classes
    (if (`self.Persistent`)
      (`LibretroCoreInstance.LoadState` (`self.LibretroCoreInstance`) "Default.sav"))))

(event `self.ReceiveEndPlay`
  (params (EndPlayReason :type "EEndPlayReason Enum" :default "Destroyed"))
  ;[0.03434 0.03434 0.03434] Unreal Delegates
  (if (`self.Persistent`)
    (`LibretroCoreInstance.SaveState` (`self.LibretroCoreInstance`) "Default.sav")))

(fn `UserConstructionScript`)